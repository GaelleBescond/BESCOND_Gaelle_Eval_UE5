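; Player controller for a 2D game that shows the player's distance from a start point on the HUD.
; On BeginPlay it creates a WBP_HUD widget and adds it to the viewport.
; Each Tick it measures the straight-line distance between the StartPosition and PlayerPosition actors, stores it in DistanceParcourue and pushes it to the HUD through ChangeDistance.
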(event EventBeginPlay
  (bind _returnvalue (UserInterface|CreateWidget "/Game/BESCOND_Gaelle/UI/WBP_HUD.WBP_HUD_C"))
  (bind _output_get (Variables|Default|SetHUD _returnvalue))
  (UserInterface|Viewport|AddtoViewport _output_get 0))

(event EventTick
  (params (DeltaSeconds :type Float%20%28single-precision%29))
  (bind _hud (Variables|Default|GetHUD))
  (bind _output_get (Variables|Default|SetDistanceParcourue (Math|Vector|Distance(Vector) (Transformation|GetActorLocation (Variables|Default|GetStartPosition)) (Transformation|GetActorLocation (Variables|Default|GetPlayerPosition)))))
  (Variables|/Game/BESCOND_Gaelle/UI/WBP_HUD.WBP_HUD_C|SetDistanceValue _hud _output_get)
  (Default|ChangeDistance _hud))

(fn ConstructionScript)